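; TV actor Blueprint that shows a live scene capture on a plane screen mesh, with an adjustable blend value.
; The construction script creates a render target for the SceneCaptureComponent2D and feeds it into a dynamic TVScreen material instance.
; Tick pushes ScreenLerp to the material's LerpAlpha parameter only when it changes; the ScreenLerp OnRep function is empty.
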(event `self.ReceiveBeginPlay`)

(event `self.ReceiveTick`
  (params (DeltaSeconds :type "Float (single-precision)"))
  (bind _screenlerp (`self.ScreenLerp`))
  (if (!= (`self.OldScreenLerp`) _screenlerp)
    (`MaterialInstanceDynamic.SetScalarParameterValue` (`self.ScreenMaterialInstance`) "LerpAlpha" _screenlerp)
    (set `self.OldScreenLerp` (`self.ScreenLerp`))))

(fn `OnRep_ScreenLerp`)

(fn `UserConstructionScript`
  (bind _returnvalue (`KismetRenderingLibrary.CreateRenderTarget2D` 256))
  (bind _output_get (set `SceneCaptureComponent2D.TextureTarget` _returnvalue (`self.SceneCaptureComponent2D`)))
  (bind _returnvalue_2 (`PrimitiveComponent.CreateDynamicMaterialInstance` (`self.Plane`) 0 "/Game/Materials/TV/TVScreen.TVScreen" "None"))
  (bind _output_get_2 (set `self.ScreenMaterialInstance` _returnvalue_2))
  (`MaterialInstanceDynamic.SetTextureParameterValue` _returnvalue_2 "Target" _output_get)
  (`MaterialInstanceDynamic.SetTextureParameterValue` _output_get_2 "Target" _output_get)
  (`MaterialInstanceDynamic.SetScalarParameterValue` _returnvalue_2 "LerpAlpha" (`self.ScreenLerp`))
  (`MaterialInstanceDynamic.SetScalarParameterValue` _output_get_2 "LerpAlpha" (`self.ScreenLerp`)))
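; Inhibitor is an interactable story pickup that grants the player the inhibitor and springs a set of guards into the level.
; On BeginPlay it hides every guard in AppearingGuards and makes their capsules ignore the Pawn channel.
; Interact sets PlayerHasInhibitor on the UESpringJamGameMode and hides the Inhibitor component, then reveals those guards, restores Pawn blocking and starts their waypoint movement.
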(event `self.ReceiveBeginPlay`
  (for _array_element (`self.AppearingGuards`)
    (`self.SetActorHiddenInGame` _array_element true)
    (`PrimitiveComponent.SetCollisionResponseToChannel` (`Character.CapsuleComponent` _array_element) "ECC_Pawn" "ECR_Ignore")))

(event `self.Interact`
  (params (interactor :type "Actor Object Reference"))
  (set `UESpringJamGameMode.playerHasInhibitor` true (cast `UESpringJamGameMode` (`GameplayStatics.GetGameMode`) :!pure true))
  (`SceneComponent.SetVisibility` (`self.Inhibitor`) false false)
  (for _array_element (`self.AppearingGuards`)
    (`self.SetActorHiddenInGame` _array_element false)
    (`PrimitiveComponent.SetCollisionResponseToChannel` (`Character.CapsuleComponent` _array_element) "ECC_Pawn" "ECR_Block")
    (`/Game/Blueprints/Guard/Guard.StartWaypointMove` _array_element)))

(fn `UserConstructionScript`)
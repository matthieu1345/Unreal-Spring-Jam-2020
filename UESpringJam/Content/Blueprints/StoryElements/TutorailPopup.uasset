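; Trigger-box actor that shows a one-time tutorial popup when the first-person character walks into it.
; On overlap, if a Popup check passes, it snaps the player's control rotation toward a look point, adds a ThoughtPopup widget with its configured text, then destroys itself.
; The construction script converts LookLocation from the box's local space into the world-space look target.
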(event `self.Box.OnComponentBeginOverlap`
  (params (OverlappedComponent :type "PrimitiveComponent Object Reference") (OtherActor :type "Actor Object Reference") (OtherComp :type "PrimitiveComponent Object Reference") (OtherBodyIndex :type Integer) (bFromSweep :type Boolean) (SweepResult :type "HitResult Structure (by ref)"))
  (bind (_asfirst_person_character _bsuccess) (cast `/Game/FirstPersonCPP/Blueprints/FirstPersonCharacter` OtherActor :!pure true))
  (if (and _bsuccess (== (`self.Popup`) null))
    (`Controller.SetControlRotation` (`Pawn.GetController` _asfirst_person_character) (`KismetMathLibrary.FindLookAtRotation` (`self.K2_GetActorLocation` _asfirst_person_character) (`self.WorldLookLocation`)))
    (bind _returnvalue (`|CreateWidget` "/Game/Blueprints/StoryElements/ThoughtPopup.ThoughtPopup_C" null (`self.TextToShow`)))
    (bind _output_get (set `self.NewVar_0` _returnvalue))
    (`UserWidget.AddToViewport` _output_get 0)
    (`self.K2_DestroyActor`)))

(fn `UserConstructionScript`
  (set `self.WorldLookLocation` (`KismetMathLibrary.TransformLocation` (`SceneComponent.K2_GetComponentToWorld` (`self.Box`)) (`self.LookLocation`))))
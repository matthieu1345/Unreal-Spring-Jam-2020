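; TextTV is an interactable TV Blueprint that shows a text popup when interacted with.
; On Interact, a passing CheckCanTeleport check creates a TextPopup widget from PopupText and removes it after a fixed delay.
; A ShowingPopup flag prevents overlapping popups during that delay.
; When the check fails, the interaction is passed to the parent class's Interact.
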(event `self.Interact`
  (params (interactor :type "Actor Object Reference"))
  (bind _returnvalue (`self.CheckCanTeleport`))
  (if _returnvalue
    (if (not (`self.ShowingPopup`))
      (bind _returnvalue_2 (`|CreateWidget` "/Game/Blueprints/TV/TextPopup.TextPopup_C" null (`self.PopupText`)))
      (bind _output_get (set `self.popup` _returnvalue_2))
      (`UserWidget.AddToViewport` _output_get 0)
      (set `self.ShowingPopup` true)
      (`KismetSystemLibrary.Delay` 5.0)
      (`Widget.RemoveFromParent` (`self.popup`))
      (set `self.ShowingPopup` false))
    (else
      (`parent.Interact` interactor))))

(fn `UserConstructionScript`
  (`parent.UserConstructionScript`))
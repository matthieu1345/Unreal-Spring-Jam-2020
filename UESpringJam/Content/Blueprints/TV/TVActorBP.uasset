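; TV actor that shows a live scene capture on its screen and can launch a signal sync minigame.
; Construction creates a render target for the SceneCapture component and feeds it into a dynamic screen material.
; Tick updates the material's LerpAlpha parameter whenever SignalStength changes.
; StartMinigame adds the TVSynchMinigame widget to the viewport and passes it this TV.
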(event `self.ReceiveBeginPlay`)

(event `self.ReceiveTick`
  (params (DeltaSeconds :type "Float (single-precision)"))
  (bind _signalstength (`self.signalStength`))
  (if (!= (`self.OldScreenLerp`) _signalstength)
    (`MaterialInstanceDynamic.SetScalarParameterValue` (`self.ScreenMaterialInstance`) "LerpAlpha" _signalstength)
    (set `self.OldScreenLerp` (`self.signalStength`))))

(event `self.StartMinigame`
  (params (interactor :type "Actor Object Reference"))
  (bind _returnvalue (`|CreateWidget` "/Game/Blueprints/TV/TVSynchMinigame.TVSynchMinigame_C"))
  (bind _output_get (set `self.MinigameUI` _returnvalue))
  (`/Game/Blueprints/TV/TVSynchMinigame.SetScreen` _output_get self)
  (`UserWidget.AddToViewport` _output_get 0))

(fn `SetVisual`
  (bind _returnvalue (`KismetRenderingLibrary.CreateRenderTarget2D` 256))
  (bind _output_get (set `SceneCaptureComponent2D.TextureTarget` _returnvalue (`self.SceneCaptureComponent2D`)))
  (bind _returnvalue_2 (`PrimitiveComponent.CreateDynamicMaterialInstance` (`self.screenmesh`) 0 "/Game/Materials/TV/TVScreen.TVScreen" "None"))
  (bind _output_get_2 (set `self.ScreenMaterialInstance` _returnvalue_2))
  (`MaterialInstanceDynamic.SetTextureParameterValue` _returnvalue_2 "Target" _output_get)
  (`MaterialInstanceDynamic.SetTextureParameterValue` _output_get_2 "Target" _output_get)
  (`MaterialInstanceDynamic.SetScalarParameterValue` _returnvalue_2 "LerpAlpha" (`self.signalStength`))
  (`MaterialInstanceDynamic.SetScalarParameterValue` _output_get_2 "LerpAlpha" (`self.signalStength`)))

(fn `UserConstructionScript`
  (`self.SetVisual`))
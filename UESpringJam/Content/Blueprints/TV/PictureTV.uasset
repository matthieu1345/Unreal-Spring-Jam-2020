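; PictureTV is a TV Blueprint variant that displays a Picture material on its screen mesh instead of using a scene capture.
; The construction script applies that material and destroys the inherited-style SceneCaptureComponent2D, which BeginPlay destroys again if still valid.
; Interacting snaps both signal values to their goals and sets signal strength to full before calling the parent Interact.
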(event `self.ReceiveBeginPlay`
  (bind _scenecapturecomponent2d (`self.SceneCaptureComponent2D`))
  (`/Engine/EditorBlueprintResources/StandardMacros.IsValid` _scenecapturecomponent2d
    (:`Is Valid`
      (`ActorComponent.K2_DestroyComponent` _scenecapturecomponent2d))))

(event `self.ReceiveTick`
  (params (DeltaSeconds :type "Float (single-precision)")))

(event `self.Interact`
  (params (interactor :type "Actor Object Reference"))
  (`self.SetSignalOne` (`self.signalFloat1Goal`))
  (`self.SetSignalTwo` (`self.signalFloat2Goal`))
  (set `self.signalStength` 1.0)
  (`parent.Interact` interactor))

(fn `UserConstructionScript`
  (`PrimitiveComponent.SetMaterial` (`self.screenmesh`) 0 (`self.Picture`))
  (`ActorComponent.K2_DestroyComponent` (`self.SceneCaptureComponent2D`)))
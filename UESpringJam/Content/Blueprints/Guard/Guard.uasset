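; Guard AI that patrols navmesh-projected local waypoints, looping or back-and-forth, and hunts the player.
; A vision cone sized from PawnSensing builds detection time, decaying out of view, until GameMode resets the player.
; PawnSensing triggers a chase toward the last seen position, then a return to the saved post or patrol.
; Both detection paths require line of sight and the player holding the inhibitor.
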(event `StartWaypointMove`
  (if (!= (`KismetArrayLibrary.Array_Length` (`self.WorldWaypoints`)) 0)
    (`|AIMoveTo` self (`|GetArrayItem` (`self.WorldWaypoints`) (`self.CurrentWaypoint`)) null 5.0 true
      (:`OnSuccess`
        (if (`self.Looping Waypoints`)
          (`self.SetLoopWaypoint`)
          (`self.StartWaypointMove`)
          (else
            (`self.SetReturnWaypoint`)
            (`self.StartWaypointMove`)))))))

(event `self.ReceiveBeginPlay`
  (`self.SetCone`)
  (set `self.GameMode` (cast `UESpringJamGameMode` (`GameplayStatics.GetGameMode`) :!pure true))
  (if (!= (`KismetArrayLibrary.Array_Length` (`self.WorldWaypoints`)) 0)
    (`self.StartWaypointMove`)))

(event `self.ReceiveTick`
  (params (DeltaSeconds :type "Float (single-precision)"))
  (bind _playerseentime (`self.PlayerSeenTime`))
  (bind _returnvalue (- _playerseentime DeltaSeconds))
  (`|ExecutionSequence`
    (:`then_0`
      (if (`self.SeesPlayer`)
        (bind _output_get (set `self.PlayerSeenTime` (+ _playerseentime DeltaSeconds)))
        (if (>= _output_get (`UESpringJamGameMode.guardDetectionTime` (`self.GameMode`)))
          (`UESpringJamGameMode.ResetPlayer` (`self.GameMode`))
          (`self.PlayerCaught`))
        (elif (>= _returnvalue 0.0)
          (set `self.PlayerSeenTime` _returnvalue)
          (else
            (set `self.PlayerSeenTime` 0.0)))))
    (:`then_1`
      (if (and (!= (`KismetArrayLibrary.Array_Length` (`self.WorldWaypoints`)) 0) (< (`KismetMathLibrary.VSizeSquared` (`self.GetVelocity`)) 1.0))
        (`self.StartWaypointMove`)))))

(event `self.Cone.OnComponentBeginOverlap`
  (params (OverlappedComponent :type "PrimitiveComponent Object Reference") (OtherActor :type "Actor Object Reference") (OtherComp :type "PrimitiveComponent Object Reference") (OtherBodyIndex :type Integer) (bFromSweep :type Boolean) (SweepResult :type "HitResult Structure (by ref)"))
  (if (== (`GameplayStatics.GetObjectClass` OtherActor) "/Game/FirstPersonCPP/Blueprints/FirstPersonCharacter.FirstPersonCharacter_C")
    (`self.CheckWatchPlayer` null
      (:`Yes`
        (set `self.SeesPlayer` true)))))

(event `self.Cone.OnComponentEndOverlap`
  (params (OverlappedComponent :type "PrimitiveComponent Object Reference") (OtherActor :type "Actor Object Reference") (OtherComp :type "PrimitiveComponent Object Reference") (OtherBodyIndex :type Integer))
  (if (== (`GameplayStatics.GetObjectClass` OtherActor) "/Game/FirstPersonCPP/Blueprints/FirstPersonCharacter.FirstPersonCharacter_C")
    (`self.CheckWatchPlayer` null
      (:`Yes`
        (set `self.SeesPlayer` false)))))

(event `PlayerCaught`
  (set `self.CaughtPlayer` true)
  (`|AIMoveTo` self (.location (`self.SeeLocation`)) null :!label _label
    (:`OnSuccess`
      (if (!= (`KismetArrayLibrary.Array_Length` (`self.WorldWaypoints`)) 0)
        (set `self.SeeLocation` (struct))
        (`self.StartWaypointMove`)
        (else
          (`self.K2_SetActorRotation` (.rotation (`self.SeeLocation`)))
          (set `self.SeeLocation` (struct)))))))

(event `self.PawnSensing.OnSeePawn`
  (params (Pawn :type "Pawn Object Reference"))
  (`self.CheckWatchPlayer` null
    (:`Yes`
      (set `self.playerLocation` (`self.K2_GetActorLocation` Pawn))
      (`self.SetFoundLocation`)
      (`|AIMoveTo` self (0.0 0.0 0.0) Pawn
        (:`then`
          (set `self.CaughtPlayer` false)
          (`KismetSystemLibrary.Delay` 1.0)
          (if (not (`self.CaughtPlayer`))
            (`|AIMoveTo` self (`self.playerLocation`) null
              (:`OnSuccess`
                (goto _label)))))))))

(fn `SetCone`
  (bind _cone (`self.Cone`))
  (bind _sightradius (`PawnSensingComponent.SightRadius` (`self.PawnSensing`)))
  (`SceneComponent.K2_SetRelativeLocation` _cone (`KismetMathLibrary.MakeVector` (/ _sightradius 2.0) 0.0 -80.0) false false)
  (`SceneComponent.SetRelativeScale3D` _cone (`KismetMathLibrary.MakeVector` 0.2 (/ (`PawnSensingComponent.PeripheralVisionAngle` (`self.PawnSensing`)) 2.8) (/ _sightradius 100.0))))

(fn `SetFoundLocation`
  (if (not (!= (.location (`self.SeeLocation`)) (0.0 0.0 0.0)))
    (set `self.SeeLocation` (`self.GetTransform`)))
  (return))

(fn `SetLoopWaypoint`
  (bind _result (`/Engine/EditorBlueprintResources/StandardMacros.IncrementInt` (`self.CurrentWaypoint`))
    (:`  `
      (if (>= _result (`KismetArrayLibrary.Array_Length` (`self.WorldWaypoints`)))
        (set `self.CurrentWaypoint` 0)))))

(fn `SetReturnWaypoint`
  (bind _returnvalue (`KismetArrayLibrary.Array_Length` (`self.WorldWaypoints`)))
  (if (`self.Backwards`)
    (bind _result (`/Engine/EditorBlueprintResources/StandardMacros.DecrementInt` (`self.CurrentWaypoint`))
      (:`  `
        (if (< _result 0)
          (set `self.CurrentWaypoint` 1)
          (set `self.Backwards` (not (`self.Backwards`)) :!label _label))))
    (else
      (bind _result_2 (`/Engine/EditorBlueprintResources/StandardMacros.IncrementInt` (`self.CurrentWaypoint`))
        (:`  `
          (if (>= _result_2 _returnvalue)
            (set `self.CurrentWaypoint` (- _returnvalue 2))
            (goto _label)))))))

(fn `UserConstructionScript`
  (`|ExecutionSequence`
    (:`then_0`
      (`KismetArrayLibrary.Array_Clear` (`self.WorldWaypoints`))
      (for _array_element (`self.Waypoints`)
        (`KismetArrayLibrary.Array_Add` (`self.WorldWaypoints`) (`NavigationSystemV1.K2_ProjectPointToNavigation` (`KismetMathLibrary.TransformLocation` (`SceneComponent.K2_GetComponentToWorld` (`self.CapsuleComponent`)) _array_element)))))
    (:`then_1`
      (`self.SetCone`))))